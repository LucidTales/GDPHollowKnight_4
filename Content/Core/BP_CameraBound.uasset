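; BP_CameraBound is a box volume that supplies camera limits on the Y/Z plane while BP_Knight overlaps it.
; Construction computes four world-space edges from the box extents, pushing any side flagged as a bridge out to a huge distance.
; Begin and end overlap add or remove it from the knight's BPCameraMovementComponent bounds list, then update that component.
; BeginPlay briefly sweeps the actor away and back to force an initial overlap.
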(event OnComponentBeginOverlap(Box)
  (params (OverlappedComponent :type Primitive%20Component%20Object%20Reference) (OtherActor :type Actor%20Object%20Reference) (OtherComp :type Primitive%20Component%20Object%20Reference) (OtherBodyIndex :type Integer) (bFromSweep :type Boolean) (SweepResult :type Hit%20Result%20Structure%20%28by%20ref%29))
  ;[0.25 0.25 0.25 0.5] Adds and removes itself from the list based on overlapping
  (bind _asbp_knight (Utilities|Casting|CastToBP_Knight OtherActor))
  (Utilities|Array|AddUnique (Variables|/Game/Core/BP_CameraMovement_Component.BP_CameraMovement_Component_C|GetCameraBounds (Variables|/Game/Core/BP_Knight.BP_Knight_C|GetBP_CameraMovement_Component _asbp_knight)) self)
  (Default|UpdateCameraBounds (Variables|/Game/Core/BP_Knight.BP_Knight_C|GetBP_CameraMovement_Component _asbp_knight)))

(event OnComponentEndOverlap(Box)
  (params (OverlappedComponent :type Primitive%20Component%20Object%20Reference) (OtherActor :type Actor%20Object%20Reference) (OtherComp :type Primitive%20Component%20Object%20Reference) (OtherBodyIndex :type Integer))
  ;[0.25 0.25 0.25 0.5] Adds and removes itself from the list based on overlapping
  (bind _asbp_knight (Utilities|Casting|CastToBP_Knight OtherActor))
  (Utilities|Array|RemoveItem (Variables|/Game/Core/BP_CameraMovement_Component.BP_CameraMovement_Component_C|GetCameraBounds (Variables|/Game/Core/BP_Knight.BP_Knight_C|GetBP_CameraMovement_Component _asbp_knight)) self)
  (Default|UpdateCameraBounds (Variables|/Game/Core/BP_Knight.BP_Knight_C|GetBP_CameraMovement_Component _asbp_knight)))

(event EventBeginPlay
  ;[0.25 0.25 0.25 0.5] Hack to ensure an overlap on begin play
  (Transformation|AddActorLocalOffset "10000.000000,0.000000, 0" true false)
  (Utilities|FlowControl|Delay 0.0)
  (Transformation|AddActorLocalOffset "-10000.000000,0.000000, 0" true false))

(fn ConstructionScript
  (bind _returnvalue (Transformation|GetActorLocation))
  (bind _box (Variables|Default|GetBox))
  (bind _returnvalue_2 (Components|Box|GetScaledBoxExtent _box))
  (bind _enumvalue (|ForEachEDirection)
    (:LoopBody
      (|SetBy-RefVar (Utilities|Select :Index _enumvalue :NewEnumerator0 (Variables|Default|GetUpBoundary) :NewEnumerator1 (Variables|Default|GetDownBoundary) :NewEnumerator2 (Variables|Default|GetLeftBoundary) :NewEnumerator3 (Variables|Default|GetRightBoundary)) (+ (Utilities|Select :Index _enumvalue :NewEnumerator0 (.z _returnvalue) :NewEnumerator1 (.z _returnvalue) :NewEnumerator2 (.y _returnvalue) :NewEnumerator3 (.y _returnvalue)) (* (select (Utilities|Select :Index _enumvalue :NewEnumerator0 (Variables|Default|GetbUpBridge) :NewEnumerator1 (Variables|Default|GetbDownBridge) :NewEnumerator2 (Variables|Default|GetbLeftBridge) :NewEnumerator3 (Variables|Default|GetbRightBridge)) 5e+07 (Utilities|Select :Index _enumvalue :NewEnumerator0 (.z _returnvalue_2) :NewEnumerator1 (.z _returnvalue_2) :NewEnumerator2 (.y _returnvalue_2) :NewEnumerator3 (.y _returnvalue_2))) (Utilities|Select :Index _enumvalue :NewEnumerator0 1.0 :NewEnumerator1 -1.0 :NewEnumerator2 -1.0 :NewEnumerator3 1.0)))))))