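; Actor component that drives the knight's side-view camera, detaching it at BeginPlay and placing it a set distance back on X.
; Each tick it eases Y and Z toward a look-direction-biased target, with interpolation speeds varying by distance and knight movement.
; The target is clamped within limits inset for a 16:9 view.
; UpdateCameraBounds resolves those limits per direction from overlapping bounds: highest layer wins, ties take the smallest absolute value.
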(event EventBeginPlay
  ;[0.25 0.25 0.25 0.5] Set references
  (bind _asbp_knight (Utilities|Casting|CastToBP_Knight (Components|GetOwner)))
  (Variables|Components|SetKnight _asbp_knight)
  (Variables|Default|SetCamera (Actor|GetComponentbyClass (Components|GetOwner) "/Script/Engine.CameraComponent"))
  ;[0.25 0.25 0.25 0.5] Detach the camera for lerp
  (Transformation|DetachFromComponent (Variables|Default|GetCamera) "KeepWorld" "KeepWorld" "KeepRelative" true)
  (Utilities|FlowControl|Delay 0.0) ; To let the detaching work
  (Transformation|SetWorldLocation (Variables|Default|GetCamera) (Math|Vector|MakeVector (+ (.x (Transformation|GetActorLocation (Variables|Components|GetKnight))) (* (Variables|Components|GetDistanceFromCharacter) -1.0)) (.y (Transformation|GetActorLocation (Variables|Components|GetKnight))) (.z (Transformation|GetActorLocation (Variables|Components|GetKnight)))) false false))

(event EventTick
  (params (DeltaSeconds :type Float%20%28single-precision%29))
  (Transformation|SetWorldLocation (Variables|Default|GetCamera) (Math|Vector|MakeVector (.x (Transformation|GetWorldLocation (Variables|Default|GetCamera))) (|YAxis) (|ZAxis)) false false))

(fn UpdateCameraBounds
  ;[0.25 0.25 0.25 0.5] Gathers boundary information from each overlaping bound
  (for _array_element (Variables|Bounds|GetCameraBounds)
    (LocalVariables|SetCurrentBound _array_element)
    ;[0.25 0.25 0.25 0.5] Each direction
    (bind _enumvalue (|ForEachEDirection)
      (:LoopBody
        ;[0.25 0.25 0.25 0.5] If that direction is considered as a potential boundary
        (if (Utilities|Select :Index _enumvalue :NewEnumerator0 (Variables|/Game/Core/BP_CameraBound.BP_CameraBound_C|GetbUp (LocalVariables|GetCurrentBound)) :NewEnumerator1 (Variables|/Game/Core/BP_CameraBound.BP_CameraBound_C|GetbDown (LocalVariables|GetCurrentBound)) :NewEnumerator2 (Variables|/Game/Core/BP_CameraBound.BP_CameraBound_C|GetbLeft (LocalVariables|GetCurrentBound)) :NewEnumerator3 (Variables|/Game/Core/BP_CameraBound.BP_CameraBound_C|GetbRight (LocalVariables|GetCurrentBound)))
          ;[0.25 0.25 0.25 0.5] If this layer is higher than the current highest, consider this as the camera bound
          (if (> (Variables|/Game/Core/BP_CameraBound.BP_CameraBound_C|GetLayer (LocalVariables|GetCurrentBound)) (Utilities|Select :Index _enumvalue :NewEnumerator0 (LocalVariables|GetLocalUpLayer) :NewEnumerator1 (LocalVariables|GetLocalDownLayer) :NewEnumerator2 (LocalVariables|GetLocalLeftLayer) :NewEnumerator3 (LocalVariables|GetLocalRightLayer)))
            (|SetBy-RefVar (Utilities|Select :Index _enumvalue :NewEnumerator0 (LocalVariables|GetLocalUpLimit) :NewEnumerator1 (LocalVariables|GetLocalDownLimit) :NewEnumerator2 (LocalVariables|GetLocalLeftLimit) :NewEnumerator3 (LocalVariables|GetLocalRightLimit)) (Utilities|Select :Index _enumvalue :NewEnumerator0 (Variables|/Game/Core/BP_CameraBound.BP_CameraBound_C|GetUpBoundary (LocalVariables|GetCurrentBound)) :NewEnumerator1 (Variables|/Game/Core/BP_CameraBound.BP_CameraBound_C|GetDownBoundary (LocalVariables|GetCurrentBound)) :NewEnumerator2 (Variables|/Game/Core/BP_CameraBound.BP_CameraBound_C|GetLeftBoundary (LocalVariables|GetCurrentBound)) :NewEnumerator3 (Variables|/Game/Core/BP_CameraBound.BP_CameraBound_C|GetRightBoundary (LocalVariables|GetCurrentBound))) :!label _label)
            (|SetBy-RefVar (Utilities|Select :Index _enumvalue :NewEnumerator0 (LocalVariables|GetLocalUpLayer) :NewEnumerator1 (LocalVariables|GetLocalDownLayer) :NewEnumerator2 (LocalVariables|GetLocalLeftLayer) :NewEnumerator3 (LocalVariables|GetLocalRightLayer)) (Variables|/Game/Core/BP_CameraBound.BP_CameraBound_C|GetLayer (LocalVariables|GetCurrentBound)))
            (else
              ;[0.25 0.25 0.25 0.5] If the layers are the same, we take the lowest value
              (if (== (Variables|/Game/Core/BP_CameraBound.BP_CameraBound_C|GetLayer (LocalVariables|GetCurrentBound)) (Utilities|Select :Index _enumvalue :NewEnumerator0 (LocalVariables|GetLocalUpLayer) :NewEnumerator1 (LocalVariables|GetLocalDownLayer) :NewEnumerator2 (LocalVariables|GetLocalLeftLayer) :NewEnumerator3 (LocalVariables|GetLocalRightLayer)))
                (if (< (Math|Float|Absolute(Float) (Utilities|Select :Index _enumvalue :NewEnumerator0 (Variables|/Game/Core/BP_CameraBound.BP_CameraBound_C|GetUpBoundary (LocalVariables|GetCurrentBound)) :NewEnumerator1 (Variables|/Game/Core/BP_CameraBound.BP_CameraBound_C|GetDownBoundary (LocalVariables|GetCurrentBound)) :NewEnumerator2 (Variables|/Game/Core/BP_CameraBound.BP_CameraBound_C|GetLeftBoundary (LocalVariables|GetCurrentBound)) :NewEnumerator3 (Variables|/Game/Core/BP_CameraBound.BP_CameraBound_C|GetRightBoundary (LocalVariables|GetCurrentBound)))) (Math|Float|Absolute(Float) (Utilities|Select :Index _enumvalue :NewEnumerator0 (LocalVariables|GetLocalUpLimit) :NewEnumerator1 (LocalVariables|GetLocalDownLimit) :NewEnumerator2 (LocalVariables|GetLocalLeftLimit) :NewEnumerator3 (LocalVariables|GetLocalRightLimit))))
                  (goto _label)))))))))
  ;[0.25 0.25 0.25 0.5] Sets the new boundaries
  (bind _enumvalue_2 (|ForEachEDirection)
    (:LoopBody
      (|SetBy-RefVar (Utilities|Select :Index _enumvalue_2 :NewEnumerator0 (Variables|Bounds|GetUpLimit) :NewEnumerator1 (Variables|Bounds|GetDownLimit) :NewEnumerator2 (Variables|Bounds|GetLeftLimit) :NewEnumerator3 (Variables|Bounds|GetRightLimit)) (Utilities|Select :Index _enumvalue_2 :NewEnumerator0 (LocalVariables|GetLocalUpLimit) :NewEnumerator1 (LocalVariables|GetLocalDownLimit) :NewEnumerator2 (LocalVariables|GetLocalLeftLimit) :NewEnumerator3 (LocalVariables|GetLocalRightLimit))))))

(event Custom|TickDebug
  ;[0.25 0.25 0.25 0.5] If distance is
)